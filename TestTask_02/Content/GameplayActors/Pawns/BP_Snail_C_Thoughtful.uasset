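; BP_Snail_C_Thoughtful is a snail pawn variant that stops moving to think after a timer runs out.
; On BeginPlay it passes its TimeToThough value to the parent's custom logic timer.
; Its AfterTimer override calls the parent, then pauses the moving timer and stops active movement on the movement component.
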(event EventBeginPlay
  (|CallParentFunction)
  (Variables|Default|SetTime_CustomLogic (Variables|Default|GetTime_ToThough)))

(fn ConstructionScript
  (|CallParentFunction))

(fn AfterTimer
  (|CallParentFunction)
  (Utilities|Time|PauseTimerbyHandle (Variables|Default|GetMovingHandle))
  (Class|NavMovementComponent|StopActiveMovement (Pawn|GetMovementComponent))
  (return))