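; BP_Snail_Base is a snail pawn base that travels to a goal location and reports when it finishes.
; The MovingtoGoal event runs an AI MoveTo toward GoalLocationW, and on success calls WhenFinish, which currently only prints a message naming the actor.
; BeginPlay and the construction script just call their parents, and nothing in this file triggers the movement or handles a failed move.
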(event EventBeginPlay
  (|CallParentFunction))

(event EventMovingtoGoal
  (AI|AIMoveTo self (Variables|Default|GetGoalLocation_W) 0 2e+01 false
    (:OnSuccess
      (Class|SnailBase|WhenFinish))))

(event EventWhenFinish
  (Development|PrintString (Utilities|String|ToString(Text) (Utilities|Text|FormatText "{Actor} is finish" self))))

(fn ConstructionScript
  (|CallParentFunction))