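; Snail pawn variant that drives its movement toward a goal with timers, extending the parent's moving and finish events.
; MovingtoGoal unpauses any valid moving timer, then sets a looping timer at TimeMovingForward and stores its handle.
; AfterTimer starts a separate one-shot timer using TimeCustomLogic.
; WhenFinish calls the parent logic, then clears and invalidates the moving timer.
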(event EventBeginPlay
  (|CallParentFunction) ; This node is disabled and will not be called.\nDrag off pins to build functionality.
)

(event EventWhenFinish
  (|CallParentFunction)
  (Utilities|Time|ClearandInvalidateTimerbyHandle (Variables|Default|GetMovingHandle)))

(event EventMovingtoGoal
  (|CallParentFunction)
  (if (Utilities|Time|IsValidTimerHandle (Variables|Default|GetMovingHandle))
    (Utilities|Time|UnpauseTimerbyHandle (Variables|Default|GetMovingHandle)))
  (bind _returnvalue (Utilities|Time|SetTimerbyEvent (EventDispatchers|CreateEvent :!event AfterTimer) (Variables|Default|GetTime_MovingForward) true))
  (Variables|Default|SetMovingHandle _returnvalue))

(fn ConstructionScript
  (|CallParentFunction))

(fn AfterTimer
  (Utilities|Time|SetTimerbyEvent (EventDispatchers|CreateEvent :!event MovingtoGoal) (Variables|Default|GetTime_CustomLogic))
  (return))